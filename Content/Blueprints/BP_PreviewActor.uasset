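; Preview actor that shows a full-body or half-body avatar mesh to a SceneCapture2D rendering only this actor's components.
; UpdateBodyType toggles the meshes, resets rotation and camera, and scales by gender, while UpdateAvatar swaps the skeletal mesh.
; RotateAvatar yaws the active mesh, and ZoomCamera steps the capture toward near or far pin components without overshooting.
; MoveCamera eases between face and full-body pins, skipping half-body avatars.
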(event `self.ReceiveBeginPlay`
  (`SceneCaptureComponent.ShowOnlyActorComponents` (`self.SceneCaptureComponent2D`) self false))

(event `Move Camera`
  (params (ToFace :type Boolean))
  (if (`|EnumInequality` (`self.BodyType`) "HalfBody")
    (bind _destination (`self.Get Destination Transform` ToFace))
    (`KismetSystemLibrary.MoveComponentTo` (`self.SceneCaptureComponent2D`) (.location _destination) (.rotation _destination) true false 0.3)))

(fn `Get Destination Transform`
  (params (ToFace :type Boolean))
  (returns (Destination :type "Transform Structure"))
  (if ToFace
    (return (`SceneComponent.GetRelativeTransform` (`self.FullBodyNearPin`)))
    (else
      (return (`SceneComponent.GetRelativeTransform` (`self.FullBodyFarPin`))))))

(fn `Get Destination Zoom Location`
  (params (Delta :type "Float (double-precision)"))
  (returns (Location :type "Vector Structure"))
  (bind _returnvalue (`|EnumEquality` (`self.BodyType`) "HalfBody"))
  (if (>= Delta 0.0)
    (if _returnvalue
      (return (`SceneComponent.RelativeLocation` (`self.HalfBodyNearPin`)))
      (else
        (return (`SceneComponent.RelativeLocation` (`self.FullBodyNearPin`)))))
    (elif _returnvalue
      (return (`SceneComponent.RelativeLocation` (`self.HalfBodyFarPin`)))
      (else
        (return (`SceneComponent.RelativeLocation` (`self.FullBodyFarPin`)))))))

(fn `Rotate Avatar`
  (params (Delta :type "Float (double-precision)"))
  (bind _returnvalue (* Delta (`self.ActorRotationSpeed`)))
  ;[1 1 1] Comment
  (if (`|EnumEquality` (`self.BodyType`) "HalfBody")
    (`SceneComponent.K2_AddRelativeRotation` (`self.HalfBodyMesh`) (`KismetMathLibrary.MakeRotator` 0.0 0.0 _returnvalue) false false)
    (else
      (`SceneComponent.K2_AddRelativeRotation` (`self.FullBodyMesh`) (`KismetMathLibrary.MakeRotator` 0.0 0.0 _returnvalue) false false))))

(fn `Update Avatar`
  (params (NewMesh :type "SkeletalMesh Object Reference"))
  (switch `EAvatarBodyType` (`self.BodyType`)
    (:`Undefined`
      (`SkinnedMeshComponent.SetSkinnedAssetAndUpdate` (`self.FullBodyMesh`) NewMesh false :!label _label))
    (:`FullBody`
      (goto _label))
    (:`HalfBody`
      (`SkinnedMeshComponent.SetSkinnedAssetAndUpdate` (`self.HalfBodyMesh`) NewMesh false))))

(fn `Update Body Type`
  (params (Gender :type "EAvatarGender Enum" :default "Undefined") (BodyType :type "EAvatarBodyType Enum" :default "Undefined"))
  (bind _fullbodymesh (`self.FullBodyMesh`))
  (bind _scenecapturecomponent2d (`self.SceneCaptureComponent2D`))
  (bind _halfbodymesh (`self.HalfBodyMesh`))
  (bind _returnvalue (`|EnumEquality` (`self.BodyType`) "HalfBody"))
  (`|ExecutionSequence`
    (:`then_0`
      ;[1 1 1] Set Body Type
      (set `self.BodyType` BodyType)
      (`SceneComponent.K2_SetRelativeRotation` :`self` (`self.FullBodyMesh`))
      (`SceneComponent.K2_SetRelativeRotation` :`self` (`self.HalfBodyMesh`))
      (`SceneComponent.SetVisibility` (`self.HalfBodyMesh`) _returnvalue false)
      (`SceneComponent.SetVisibility` (`self.FullBodyMesh`) (not _returnvalue) false)
      (if _returnvalue
        (`SceneComponent.K2_SetRelativeTransform` _scenecapturecomponent2d (`SceneComponent.GetRelativeTransform` (`self.HalfBodyNearPin`)) false false)
        (else
          (`SceneComponent.K2_SetRelativeTransform` _scenecapturecomponent2d (`SceneComponent.GetRelativeTransform` (`self.FullBodyFarPin`)) false false))))
    (:`then_1`
      ;[1 1 1] Set Gender
      (if (`|EnumEquality` Gender "Feminine")
        (`SceneComponent.SetRelativeScale3D` _fullbodymesh (1.07 1.07 1.07))
        (`SceneComponent.SetRelativeScale3D` _halfbodymesh (1.07 1.07 1.07))
        (else
          (`SceneComponent.SetRelativeScale3D` _fullbodymesh (1.0 1.0 1.0))
          (`SceneComponent.SetRelativeScale3D` _halfbodymesh (1.0 1.0 1.0)))))))

(fn `UserConstructionScript`)

(fn `Zoom Camera`
  (params (Delta :type "Float (double-precision)"))
  (bind _location (.location (`SceneComponent.GetRelativeTransform` (`self.SceneCaptureComponent2D`))))
  (bind _location_2 (`self.Get Destination Zoom Location` Delta))
  (`SceneComponent.K2_SetRelativeTransform` (`self.SceneCaptureComponent2D`) (`KismetMathLibrary.MakeTransform` (- _location (* (`KismetMathLibrary.Normal` (- _location _location_2)) (`KismetMathLibrary.FMin` (`KismetMathLibrary.Abs` (* Delta (`self.ActorZoomSpeed`))) (`KismetMathLibrary.Vector_Distance` _location _location_2)))) (.rotation (`SceneComponent.GetRelativeTransform` (`self.SceneCaptureComponent2D`)))) false false))
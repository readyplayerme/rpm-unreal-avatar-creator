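; BI_RPM_PreviewAvatar is a Blueprint Interface for controlling an RPM avatar preview.
; It declares calls to move the camera toward or away from the face, zoom it and rotate the avatar.
; Further calls update the body type by gender or swap in a skeletal mesh.
; Getters for a render material and render target size suggest the preview is displayed through a render target.
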(fn `GetRenderMaterial`
  (returns (Material :type "MaterialInterface Object Reference"))
  (return null))

(fn `GetRenderTargetSize`
  (returns (Size :type "Vector2D Structure"))
  (return (0.0 0.0)))

(fn `MoveCamera`
  (params (ToFace :type Boolean)))

(fn `RotateAvatar`
  (params (Delta :type "Float (double-precision)"))
  (return))

(fn `UpdateAvatar`
  (params (SkeletalMesh :type "SkeletalMesh Object Reference"))
  (return))

(fn `UpdateBodyType`
  (params (Gender :type "EAvatarGender Enum" :default "Undefined") (BodyType :type "EAvatarBodyType Enum" :default "Undefined"))
  (return))

(fn `ZoomCamera`
  (params (Delta :type "Float (double-precision)"))
  (return))
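; Avatar preview actor (RPM) that captures only its own components with a SceneCapture2D and supplies a render material and target size.
; It shows a full-body or half-body mesh by body type, with yaw rotation on either.
; Near and far pin components define camera framing for zoom and for the eased face/body move, which is full-body only.
; Swapped-in meshes are scaled using gender and a clamped ratio against the initial full-body mesh bounds.
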(event `self.ReceiveBeginPlay`
  (`SceneCaptureComponent.ShowOnlyActorComponents` (`self.SceneCaptureComponent2D`) self false)
  (`self.SetInitialMeshHeights`))

(event `/RpmAvatarCreator/Blueprints/BI_RPM_PreviewAvatar.MoveCamera`
  (params (ToFace :type Boolean))
  (if (`|EnumInequality` (`self.BodyType`) "HalfBody")
    (bind _destination (`self.Get Destination Transform` ToFace))
    (`KismetSystemLibrary.MoveComponentTo` (`self.SceneCaptureComponent2D`) (.location _destination) (.rotation _destination) true false 0.3)))

(event `/RpmAvatarCreator/Blueprints/BI_RPM_PreviewAvatar.UpdateAvatar`
  (params (SkeletalMesh :type "SkeletalMesh Object Reference"))
  (`self.Update Avatar Impl` SkeletalMesh))

(event `/RpmAvatarCreator/Blueprints/BI_RPM_PreviewAvatar.UpdateBodyType`
  (params (Gender :type "EAvatarGender Enum" :default "Undefined") (BodyType :type "EAvatarBodyType Enum" :default "Undefined"))
  (`self.Update Body Type Impl` Gender BodyType))

(event `/RpmAvatarCreator/Blueprints/BI_RPM_PreviewAvatar.RotateAvatar`
  (params (Delta :type "Float (single-precision)"))
  (`self.Rotate Avatar Impl` Delta))

(event `/RpmAvatarCreator/Blueprints/BI_RPM_PreviewAvatar.ZoomCamera`
  (params (Delta :type "Float (single-precision)"))
  (`self.Zoom Camera Impl` Delta))

(fn `Get Destination Transform`
  (params (ToFace :type Boolean))
  (returns (Destination :type "Transform Structure"))
  (if ToFace
    (return (`SceneComponent.GetRelativeTransform` (`self.FullBodyNearPin`)))
    (else
      (return (`SceneComponent.GetRelativeTransform` (`self.FullBodyFarPin`))))))

(fn `Get Destination Zoom Location`
  (params (Delta :type "Float (double-precision)"))
  (returns (Location :type "Vector Structure"))
  (bind _returnvalue (`|EnumEquality` (`self.BodyType`) "HalfBody"))
  (if (>= Delta 0.0)
    (if _returnvalue
      (return (`SceneComponent.RelativeLocation` (`self.HalfBodyNearPin`)))
      (else
        (return (`SceneComponent.RelativeLocation` (`self.FullBodyNearPin`)))))
    (elif _returnvalue
      (return (`SceneComponent.RelativeLocation` (`self.HalfBodyFarPin`)))
      (else
        (return (`SceneComponent.RelativeLocation` (`self.FullBodyFarPin`)))))))

(fn `GetRenderMaterial`
  (returns (Material :type "MaterialInterface Object Reference"))
  (return "/RpmAvatarCreator/Materials/M_RPM_PreviewRenderMaterial.M_RPM_PreviewRenderMaterial"))

(fn `GetRenderTargetSize`
  (returns (Size :type "Vector2D Structure"))
  ;[1 1 1] Return Render Target Dimentions
  (return (1536.0 1024.0)))

(fn `Rotate Avatar Impl`
  (params (Delta :type "Float (double-precision)"))
  (bind _returnvalue (* Delta (`self.ActorRotationSpeed`)))
  ;[1 1 1] Comment
  (if (`|EnumEquality` (`self.BodyType`) "HalfBody")
    (`SceneComponent.K2_AddRelativeRotation` (`self.HalfBodyMesh`) (`KismetMathLibrary.MakeRotator` 0.0 0.0 _returnvalue) false false)
    (else
      (`SceneComponent.K2_AddRelativeRotation` (`self.FullBodyMesh`) (`KismetMathLibrary.MakeRotator` 0.0 0.0 _returnvalue) false false))))

(fn `SetInitialMeshHeights`
  (set `self.InitialFullBodyHeight` (.z (`.BoxExtent` (`KismetMathLibrary.BreakBoxSphereBounds` (`SkeletalMesh.GetBounds` (`RpmAvatarCreatorFunctionLibrary.GetSkeletalMeshFromComponent` (`self.FullBodyMesh`)))))))
  (set `self.InitialHalfBodyHeight` (.z (`.BoxExtent` (`KismetMathLibrary.BreakBoxSphereBounds` (`SkeletalMesh.GetBounds` (`RpmAvatarCreatorFunctionLibrary.GetSkeletalMeshFromComponent` (`self.FullBodyMesh`))))))))

(fn `SetMeshScale`
  (params (MeshComponent :type "SkeletalMeshComponent Object Reference") (InitialHeight :type "Float (double-precision)"))
  (locals (Scale :type "Float (double-precision)" :default 1.0))
  (bind _meshscalethreshold (`self.MeshScaleThreshold`))
  (bind _returnvalue (- 1.0 _meshscalethreshold))
  (bind _returnvalue_2 (+ 1.0 _meshscalethreshold))
  (bind _returnvalue_3 (/ InitialHeight (.z (`.BoxExtent` (`KismetMathLibrary.BreakBoxSphereBounds` (`SkeletalMesh.GetBounds` (`RpmAvatarCreatorFunctionLibrary.GetSkeletalMeshFromComponent` MeshComponent)))))))
  (`|ExecutionSequence`
    (:`then_0`
      ;[1 1 1] Set Female Mesh Scale
      (if (`|EnumEquality` (`self.Gender`) "Feminine")
        (set `local.Scale` 1.05)))
    (:`then_1`
      ;[1 1 1] Clamp Scale
      (if (not (`KismetMathLibrary.InRange_FloatFloat` _returnvalue_3 _returnvalue _returnvalue_2))
        (set `local.Scale` (`KismetMathLibrary.FClamp` _returnvalue_3 _returnvalue _returnvalue_2))))
    (:`then_2`
      ;[1 1 1] Set Final Scale
      (`SceneComponent.SetRelativeScale3D` MeshComponent (`KismetMathLibrary.Conv_DoubleToVector` (`local.Scale`))))))

(fn `Update Avatar Impl`
  (params (NewMesh :type "SkeletalMesh Object Reference"))
  (bind _fullbodymesh (`self.FullBodyMesh`))
  (bind _halfbodymesh (`self.HalfBodyMesh`))
  (switch `EAvatarBodyType` (`self.BodyType`)
    (:`Undefined`
      (`SkinnedMeshComponent.SetSkinnedAssetAndUpdate` _fullbodymesh NewMesh false :!label _label)
      (`self.SetMeshScale` _fullbodymesh (`self.InitialFullBodyHeight`)))
    (:`FullBody`
      (goto _label))
    (:`HalfBody`
      (`SkinnedMeshComponent.SetSkinnedAssetAndUpdate` _halfbodymesh NewMesh false)
      (`self.SetMeshScale` _halfbodymesh (`self.InitialHalfBodyHeight`)))))

(fn `Update Body Type Impl`
  (params (Gender :type "EAvatarGender Enum" :default "Undefined") (BodyType :type "EAvatarBodyType Enum" :default "Undefined"))
  (bind _scenecapturecomponent2d (`self.SceneCaptureComponent2D`))
  (bind _returnvalue (`|EnumEquality` (`self.BodyType`) "HalfBody"))
  (set `self.Gender` Gender)
  ;[1 1 1] Set Body Type
  (set `self.BodyType` BodyType)
  (`SceneComponent.K2_SetRelativeRotation` :`self` (`self.FullBodyMesh`))
  (`SceneComponent.K2_SetRelativeRotation` :`self` (`self.HalfBodyMesh`))
  (`SceneComponent.SetVisibility` (`self.HalfBodyMesh`) _returnvalue false)
  (`SceneComponent.SetVisibility` (`self.FullBodyMesh`) (not _returnvalue) false)
  (if _returnvalue
    (`SceneComponent.K2_SetRelativeTransform` _scenecapturecomponent2d (`SceneComponent.GetRelativeTransform` (`self.HalfBodyNearPin`)) false false)
    (else
      (`SceneComponent.K2_SetRelativeTransform` _scenecapturecomponent2d (`SceneComponent.GetRelativeTransform` (`self.FullBodyFarPin`)) false false))))

(fn `UserConstructionScript`)

(fn `Zoom Camera Impl`
  (params (Delta :type "Float (double-precision)"))
  (bind (_returnvalue_location _returnvalue_rotation) (`KismetMathLibrary.BreakTransform` (`SceneComponent.GetRelativeTransform` (`self.SceneCaptureComponent2D`))))
  (bind _location (`self.Get Destination Zoom Location` Delta))
  (`SceneComponent.K2_SetRelativeTransform` (`self.SceneCaptureComponent2D`) (`KismetMathLibrary.MakeTransform` (- _returnvalue_location (* (`KismetMathLibrary.Normal` (- _returnvalue_location _location)) (`KismetMathLibrary.FMin` (`KismetMathLibrary.Abs` (* Delta (`self.ActorZoomSpeed`))) (`KismetMathLibrary.Vector_Distance` _returnvalue_location _location)))) _returnvalue_rotation) false false))